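; Pressure plate actor that swings a referenced door open while something overlaps it.
; Trigger overlap plays the SafeDoorOpen timeline and any actor end overlap reverses it, with IsPlayingForward guarding repeat calls.
; The timeline's single DoorRot track drives both the door's relative yaw and, scaled down and negated, the plate's own relative Z for the sinking press.
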(event OnComponentBeginOverlap(trigger)
  (params (OverlappedComponent :type Primitive%20Component%20Object%20Reference) (OtherActor :type Actor%20Object%20Reference) (OtherComp :type Primitive%20Component%20Object%20Reference) (OtherBodyIndex :type Integer) (bFromSweep :type Boolean) (SweepResult :type Hit%20Result%20Structure%20%28by%20ref%29))
  ;[1 1 1] Determine Case
  (if (not (Variables|Default|GetIsPlayingForward))
    (Variables|Default|SetIsPlayingForward true)
    (bind _doorrot (Timeline|SafeDoorOpen Play)
      (:Update
        (Transformation|SetActorRelativeRotation (Variables|Default|GetDoorRef) (Math|Rotator|MakeRotator 0.0 0.0 _doorrot))
        (Transformation|SetActorRelativeLocation (/ (Math|Vector|MakeVector 0.0 0.0 _doorrot) "1.000000,1.000000,-30.000000"))))))

(event Collision|EventActorEndOverlap
  (params (OtherActor :type Actor%20Object%20Reference))
  ;[1 1 1] Determine Case
  (if (Variables|Default|GetIsPlayingForward)
    (Variables|Default|SetIsPlayingForward false)
    (bind _doorrot (Timeline|SafeDoorOpen Reverse)
      (:Update
        (Transformation|SetActorRelativeRotation (Variables|Default|GetDoorRef) (Math|Rotator|MakeRotator 0.0 0.0 _doorrot))
        (Transformation|SetActorRelativeLocation (/ (Math|Vector|MakeVector 0.0 0.0 _doorrot) "1.000000,1.000000,-30.000000"))))))

(fn ConstructionScript)