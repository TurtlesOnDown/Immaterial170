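; Actor for a 3D hand menu, hosting a w_HandMenu widget through its Menu component and feeding it motion controller thumb input.
; Every Tick it casts the component's user widget to w_HandMenu and checks the left and right active flags independently.
; For each active hand, it copies that controller's thumb X and Y axes into the widget's matching hand variables.
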(event EventBeginPlay)

(event Collision|EventActorBeginOverlap
  (params (OtherActor :type Actor%20Object%20Reference)))

(event EventTick
  (params (DeltaSeconds :type Float%20%28single-precision%29))
  ;[1 1 1] Send Input to the correct hand only if a menu is active.
  (bind _asw_hand_menu (Utilities|Casting|CastTow_HandMenu (UserInterface|GetUserWidgetObject (Variables|Default|GetMenu))))
  (Utilities|FlowControl|Sequence
    (:then_0
      (if (Variables|/Game/Blueprints/Menu/w_HandMenu.w_HandMenu_C|GetActiveL _asw_hand_menu)
        (Variables|/Game/Blueprints/Menu/w_HandMenu.w_HandMenu_C|SetLeftHandX _asw_hand_menu (Input|AxisValues|GetMotionControllerThumbLeft_X))
        (Variables|/Game/Blueprints/Menu/w_HandMenu.w_HandMenu_C|SetLeftHandY _asw_hand_menu (Input|AxisValues|GetMotionControllerThumbLeft_Y))))
    (:then_1
      (if (Variables|/Game/Blueprints/Menu/w_HandMenu.w_HandMenu_C|GetActiveR _asw_hand_menu)
        (Variables|/Game/Blueprints/Menu/w_HandMenu.w_HandMenu_C|SetRightHandX _asw_hand_menu (Input|AxisValues|GetMotionControllerThumbRight_X))
        (Variables|/Game/Blueprints/Menu/w_HandMenu.w_HandMenu_C|SetRightHandY _asw_hand_menu (Input|AxisValues|GetMotionControllerThumbRight_Y))))))

(fn ConstructionScript)