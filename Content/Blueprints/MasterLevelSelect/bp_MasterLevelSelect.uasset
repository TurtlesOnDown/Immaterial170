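; bp_MasterLevelSelect handles transfers between streamed levels through its Transfer event, ignoring requests for the current level.
; A DoOnce blocks overlapping transfers while the target level streams in and audio plays.
; A timeline drives a distance multiplier in a material parameter collection, forward or reversed depending on ToLimbo, as the transition effect.
; When it finishes, the old level unloads, GameInstance's CurrentLevel updates and the gate resets.
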(event EventTransfer
  (params (LeveltoLoad :type Name) (ToLimbo :type Boolean) (TransitionType :type Integer))
  (bind _returnvalue (Game|GetGameInstance))
  (bind _asbp_game_instance (Utilities|Casting|CastTobp_GameInstance _returnvalue))
  (if (not (Utilities|Name|Equal(Name) LeveltoLoad (Variables|/Game/Blueprints/GameInstance/bp_GameInstance.bp_GameInstance_C|GetCurrentLevel (.AsBp%20Game%20Instance (Utilities|Casting|CastTobp_GameInstance (Game|GetGameInstance))))))
    (Utilities|FlowControl|DoOnce false :!label _label
      (:Completed
        (Variables|Default|SetLeveltoLoad LeveltoLoad)
        (Variables|Default|SetToLimbo ToLimbo)
        (switch int TransitionType
          (:0
            (Game|LoadStreamLevel(byName) (Variables|Default|GetLeveltoLoad) true)
            (Audio|Components|Audio|Play (Variables|Default|GetAudio) 0.0)
            (if (Variables|Default|GetToLimbo)
              (bind _fadedistance (Timeline|Timeline_0 PlayFromStart)
                (:Update
                  (Rendering|Material|SetScalarParameterValue "/Game/Materials/mpc_Distances.Mpc_Distances" "distanceMultipler" _fadedistance :!class /Script/Engine.KismetMaterialLibrary))
                (:Finished
                  (Game|UnloadStreamLevel(byName) (Variables|/Game/Blueprints/GameInstance/bp_GameInstance.bp_GameInstance_C|GetCurrentLevel _asbp_game_instance))
                  (Variables|/Game/Blueprints/GameInstance/bp_GameInstance.bp_GameInstance_C|SetCurrentLevel _asbp_game_instance (Variables|Default|GetLeveltoLoad))
                  (goto _label Reset)))
              (else
                (Timeline|Timeline_0 ReverseFromEnd)))))))))

(fn ConstructionScript)