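; Music cue Blueprint that crossfades between two audio components when the game instance's current level is "level3_Gold_Move".
; Tick polls that level name on bp_GameInstance and, on a match, fades out Audio1 over half a second.
; While Audio1 is still playing, each tick also activates and fades in Audio over one second and prints its world location for debugging.
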(event EventTick
  (params (DeltaSeconds :type Float%20%28single-precision%29))
  (if (Utilities|Name|Equal(Name) (Variables|/Game/Blueprints/GameInstance/bp_GameInstance.bp_GameInstance_C|GetCurrentLevel (.AsBp%20Game%20Instance (Utilities|Casting|CastTobp_GameInstance (Game|GetGameInstance)))) "level3_Gold_Move")
    (Audio|Components|Audio|FadeOut (Variables|Default|GetAudio1) 0.5 0.0 :!class /Script/Engine.AudioComponent)
    (if (Audio|Components|Audio|IsPlaying (Variables|Default|GetAudio1))
      (Components|Activation|Activate (Variables|Default|GetAudio) false)
      (Audio|Components|Audio|FadeIn (Variables|Default|GetAudio) 1.0 1.0 0.0 :!class /Script/Engine.AudioComponent)
      (Development|PrintString (Utilities|String|ToString(Vector) (Transformation|GetWorldLocation (Variables|Default|GetAudio)))))))

(fn ConstructionScript)